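; Cube64_Blueprint is an unfinished interactable actor with a forward line trace and a disconnected life-reduction step.
; Every Tick it traces 500 units ahead on the Visibility channel with debug drawing.
; A trace hit or an Interact event casts the player character to DefaultCharacter, then does nothing further.
; The node meant to subtract 5 from LifeActually is unwired, so it never runs.
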(event `self.ReceiveTick`
  (params (DeltaSeconds :type "Float (single-precision)"))
  (bind _returnvalue (`self.K2_GetActorLocation`))
  (bind (_outhit _returnvalue_2) (`KismetSystemLibrary.LineTraceSingle` :`Start` _returnvalue :`End` (+ _returnvalue (* (`self.GetActorForwardVector`) 500.0)) :`TraceChannel` "TraceTypeQuery1" :`DrawDebugType` "ForOneFrame"))
  (if _returnvalue_2
    (bind _asdefault_character (cast `/Game/Blueprints/DefaultCharacter` (`GameplayStatics.GetPlayerCharacter` 0) :!label _label))))

(event `/Game/Blueprints/Interfaces/I_Interaction.Interact`
  (params (Character :type "/Game/Blueprints/DefaultCharacter Object Reference"))
  (goto _label))

(fn `UserConstructionScript`)