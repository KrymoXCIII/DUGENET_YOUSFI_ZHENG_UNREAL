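; Moving spikes trap actor that stays idle until an Interact event switches it on.
; Once active, Tick either pops it up once along local Z when OnlyOnce is set, using the First flag, or slides it along local X every frame.
; Movement uses fixed, unswept local offsets with no delta-time scaling, so the sliding speed follows frame rate and has no stop condition.
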(event `self.ReceiveActorBeginOverlap`
  (params (OtherActor :type "Actor Object Reference")))

(event `self.ReceiveTick`
  (params (DeltaSeconds :type "Float (single-precision)"))
  (if (`self.Active`)
    (if (`self.OnlyOnce`)
      (if (`self.First`)
        (`self.K2_AddActorLocalOffset` (0.0 0.0 70.0))
        (set `self.First` false))
      (else
        (`self.K2_AddActorLocalOffset` (10.0 0.0 0.0))))))

(event `/Game/Blueprints/Interfaces/I_Interaction.Interact`
  (params (Character :type "/Game/Blueprints/DefaultCharacter Object Reference"))
  (set `self.Active` true))

(fn `UserConstructionScript`)