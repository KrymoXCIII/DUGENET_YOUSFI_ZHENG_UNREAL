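; Player character with movement, look, jump and timeline-smoothed capsule crouch, plus life and countdown survival rules.
; BeginPlay initializes life, adds the HUD and starts a looping timer on a named function, presumably DecreaseLife, which never lowers life to zero.
; Any overlap costs life immediately, with a Delay loop repeating damage on Traps.
; Tick runs a Delay-gated countdown, pausing into GameOver when time or life hits exactly zero; A fires a debug trace.
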(event `self.ReceiveActorBeginOverlap`
  (params (OtherActor :type "Actor Object Reference"))
  (`|ExecutionSequence`
    (:`then_0`
      (set `self.Life_Actually` (- (`self.Life_Actually`) 5.0) :!label _label)
      (if (`self.IsOverlappingActor` (cast `/Game/Blueprints/Trap` OtherActor :!pure true))
        (`KismetSystemLibrary.Delay` 0.5 :!label _label_2)
        (goto _label)))
    (:`then_1`
      (goto _label_2))))

(event `self.ReceiveBeginPlay`
  (`|ExecutionSequence`
    (:`then_0`
      (set `self.CapsuleHalfHeight` (`CapsuleComponent.CapsuleHalfHeight` (`self.CapsuleComponent`))))
    (:`then_1`
      (`self.Def init stat perso`))
    (:`then_2`
      (`self.Def Base stat Actually`))
    (:`then_3`
      (`KismetSystemLibrary.K2_SetTimer` self (`self.decrement_life_name`) 5.0 true))
    (:`then_4`
      (bind _returnvalue (`|CreateWidget` "/Game/Blueprints/UserInterface.UserInterface_C"))
      (`UserWidget.AddToViewport` _returnvalue 0))))

(event `InputAxis|Fw/Bw`
  (params (AxisValue :type "Float (single-precision)"))
  ;[0.4479 0.4357 0.4115] DEPLACEMENTS
  (`self.AddMovementInput` (`KismetMathLibrary.GetForwardVector` (`KismetMathLibrary.MakeRotator` 0.0 (.pitch (`self.GetControlRotation`)) (.yaw (`self.GetControlRotation`)))) AxisValue))

(event `InputAxis|R/L`
  (params (AxisValue :type "Float (single-precision)"))
  ;[0.4479 0.4357 0.4115] DEPLACEMENTS
  (`self.AddMovementInput` (`KismetMathLibrary.GetRightVector` (`KismetMathLibrary.MakeRotator` 0.0 (.pitch (`self.GetControlRotation`)) (.yaw (`self.GetControlRotation`)))) AxisValue))

(event `InputAxis|LU/LD`
  (params (AxisValue :type "Float (single-precision)"))
  ;[0.1117 1 0.4183] ROTATIONS
  (`self.AddControllerPitchInput` (`KismetMathLibrary.FClamp` AxisValue -5.0 5.0)))

(event `InputAxis|LR/LL`
  (params (AxisValue :type "Float (single-precision)"))
  ;[0.1117 1 0.4183] ROTATIONS
  (`self.AddControllerYawInput` (`KismetMathLibrary.FClamp` AxisValue -5.0 5.0)))

(event `InputAction|JUMP`
  (params (Key :type "Key Structure"))
  ;[1 1 1] SAUT ET S'ACCROUPIR
  (:`Pressed`
    (`self.Jump`)))

(event `InputAction|CROUCH`
  (params (Key :type "Key Structure"))
  ;[1 1 1] SAUT ET S'ACCROUPIR
  (:`Pressed`
    (`self.StartCrouch`))
  (:`Released`
    (`self.StopCrouch`)))

(event `StartCrouch`
  (set `self.IsCrouched` true)
  (bind (_direction _lerpvalue) (`Timeline|CrouchSmooth` :!label _label_3)
    (:`Update`
      (`CapsuleComponent.SetCapsuleHalfHeight` (`self.CapsuleComponent`) (`KismetMathLibrary.Lerp` (`self.CapsuleHalfHeight`) (`CharacterMovementComponent.CrouchedHalfHeight` (`self.CharacterMovement`)) _lerpvalue) true))))

(event `StopCrouch`
  (set `self.IsCrouched` false)
  (goto _label_3 :!via `Reverse`))

(event `Key|A`
  (params (Key :type "Key Structure"))
  (:`Pressed`
    (`KismetSystemLibrary.LineTraceSingle` :`Start` (`self.K2_GetActorLocation`) :`End` (* (`KismetMathLibrary.GetForwardVector` (`self.GetControlRotation`)) 150.0) :`TraceChannel` "TraceTypeQuery1" :`DrawDebugType` "Persistent")
    (`KismetSystemLibrary.PrintString` "Hello")))

(event `self.ReceiveTick`
  (params (DeltaSeconds :type "Float (single-precision)"))
  (`|ExecutionSequence`
    (:`then_0`
      (`KismetSystemLibrary.Delay` 1.0)
      (if (== (`self.seconds`) 0)
        (if (== (`self.minute`) 0)
          (bind _returnvalue (`|CreateWidget` "/Game/Blueprints/GameOver.GameOver_C"))
          (`UserWidget.AddToViewport` _returnvalue 0)
          (set `PlayerController.bShowMouseCursor` true (`GameplayStatics.GetPlayerController` 0))
          (`GameplayStatics.SetGamePaused` true)
          (else
            (set `self.seconds` 59)
            (set `self.minute` (- (`self.minute`) 1))))
        (else
          (set `self.seconds` (- (`self.seconds`) 1)))))
    (:`then_1`
      (if (== (`self.Life_Actually`) 0.0)
        (bind _returnvalue_2 (`|CreateWidget` "/Game/Blueprints/GameOver.GameOver_C"))
        (`UserWidget.AddToViewport` _returnvalue_2 0)
        (set `PlayerController.bShowMouseCursor` true (`GameplayStatics.GetPlayerController` 0))
        (`GameplayStatics.SetGamePaused` true)))))

(fn `decrease life`
  (bind _returnvalue (`KismetMathLibrary.FClamp` (- (`self.Life_Actually`) (`self.Life_decrement`)) 0.0 (`self.Life_base`)))
  (if (not (<= _returnvalue 0.0))
    (set `self.Life_Actually` _returnvalue)))

(fn `Def Base stat Actually`
  (set `self.Life_Actually` (`self.Life_base`)))

(fn `Def init stat perso`
  (set `self.Life_base` 100.0))

(fn `UserConstructionScript`)