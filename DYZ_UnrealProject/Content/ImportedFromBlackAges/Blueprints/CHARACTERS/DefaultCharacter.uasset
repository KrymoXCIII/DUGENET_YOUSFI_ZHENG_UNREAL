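; Player character with first/third-person camera switching, movement, tagged-item pickup and drop, and montage-driven melee attacks that lock yaw.
; On overlap, a striking zombie's right hand drains PLAYERHEALTH, and every overlapped actor receives an interact message.
; BeginPlay creates the HUD and starts a looping life timer by function name.
; Death and ragdoll functions are never called here; smooth crouch, stat initialization, axe spawning and weapon hitbox logic are disconnected.
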(event `self.ReceiveActorBeginOverlap`
  (params (OtherActor :type "Actor Object Reference"))
  ;[0.219 1 0] BEGIN OVERLAP
  (`|ExecutionSequence`
    (:`then_0`
      (bind _aszombie_character (cast `/Game/Blueprints/CHARACTERS/ZombieCharacter` OtherActor))
      (if (`/Game/Blueprints/CHARACTERS/ZombieCharacter.isStriking` _aszombie_character)
        (if (`PrimitiveComponent.IsOverlappingActor` (`/Game/Blueprints/CHARACTERS/ZombieCharacter.RightHand` _aszombie_character) self)
          (`/Engine/EditorBlueprintResources/StandardMacros.DoOnce` false :!label _label
            (:`Completed`
              (`KismetSystemLibrary.PrintString` "ZOMBIE ATTACK" true true (struct :`R` 1.0 :`G` 0.009182 :`A` 1.0))
              (set `self.PLAYERHEALTH` (`KismetMathLibrary.FClamp` (- (`self.PLAYERHEALTH`) 20.0) 0.0 100.0))
              (bind _returnvalue (`self.PlayAnimMontage` "/Game/ANIMS/ZOMBIE/RETARGETED/zombie_impact_Montage.zombie_impact_Montage"))
              (`KismetSystemLibrary.Delay` _returnvalue)
              (goto _label :!via `Reset`))))))
    (:`then_1`
      (message `/Game/Blueprints/Interfaces/I_Interaction.Interact` OtherActor self))))

(event `self.ReceiveTick`
  (params (DeltaSeconds :type "Float (single-precision)"))
  ;[1 0.8557 0] EVENT TICK
  (`|ExecutionSequence`))

(event `self.ReceiveBeginPlay`
  (bind _returnvalue (`GameplayStatics.GetPlayerController` 0))
  ;[0 0.007759 1] BEGINPLAY
  (`|ExecutionSequence`
    (:`then_0`
      (set `self.CapsuleHalfHeight` (`CapsuleComponent.CapsuleHalfHeight` (`self.CapsuleComponent`))))
    (:`then_1`
      (set `self.PLAYERHEALTH` 100.0))
    (:`then_3`
      (`KismetSystemLibrary.K2_SetTimer` self (`self.decrement_life_name`) 5.0 true))
    (:`then_4`
      (bind _returnvalue_2 (`|CreateWidget` "/Game/UI/WBP_HUD.WBP_HUD_C" _returnvalue))
      (`UserWidget.AddToViewport` _returnvalue_2 0)
      (`WidgetBlueprintLibrary.SetInputMode_GameOnly` _returnvalue))))

(event `InputAction|PICKUP/INTERACT`
  (params (Key :type "Key Structure"))
  ;[0.3385 0.08093 0.07756] PICKUP/INTERACT
  (:`Pressed`
    (if (not (`self.isHolding`))
      (for _array_element (`self.GetOverlappingActors` "/Script/Engine.Actor")
        (if (`self.ActorHasTag` _array_element "PICKUPABLE")
          ;;[0.2251 1 0.1025] PICKUP
          (bind _output_get (set `self.HELD_ITEM` _array_element))
          (`self.K2_AttachToComponent` _output_get (`self.Mesh`) "AxeHandSocket" "SnapToTarget" "SnapToTarget" "SnapToTarget" true)
          (set `self.isHolding` true)
          (break))))))

(event `InputAction|WALK`
  (params (Key :type "Key Structure"))
  ;[0 0.3762 0.6458] DEPLACEMENTS
  (:`Pressed`
    (set `CharacterMovementComponent.MaxWalkSpeed` 300.0 (`self.CharacterMovement`)))
  (:`Released`
    (set `CharacterMovementComponent.MaxWalkSpeed` 500.0 (`self.CharacterMovement`))))

(event `InputAxis|FW/BW`
  (params (AxisValue :type "Float (single-precision)"))
  ;[0 0.3762 0.6458] DEPLACEMENTS
  (`self.AddMovementInput` (`KismetMathLibrary.GetForwardVector` (`KismetMathLibrary.MakeRotator` 0.0 0.0 (.yaw (`self.GetControlRotation`)))) AxisValue))

(event `Key|LeftMouseButton`
  (params (Key :type "Key Structure"))
  ;[1 0 0] ATTACK
  (:`Pressed`
    (if (`self.isHolding`)
      (set `self.isStriking` true)
      (`|PlayMontage` (`self.Mesh`) "/Game/ANIMS/ZOMBIE/RETARGETED/PLAYER_attack_MontageATTACK1.PLAYER_attack_MontageATTACK1"
        (:`then`
          (`|ExecutionSequence`
            (:`then_1`
              ;[0.5781 0.01093 0] BLOCK CAMERA DURING ATTACK
              (bind _asdefault_character (cast `/Game/ImportedFromBlackAges/Blueprints/CHARACTERS/DefaultCharacter` (`GameplayStatics.GetPlayerCharacter` 0)))
              (set `Pawn.bUseControllerRotationYaw` true _asdefault_character)
              (`KismetSystemLibrary.Delay` 1.5)
              (if (not (`self.isFPS`))
                (set `Pawn.bUseControllerRotationYaw` false _asdefault_character)))))
        (:`OnCompleted`
          (set `self.isStriking` false))))))

(event `InputAxis|RIGHT/LEFT`
  (params (AxisValue :type "Float (single-precision)"))
  ;[0 0.3762 0.6458] DEPLACEMENTS
  (`self.AddMovementInput` (`KismetMathLibrary.GetRightVector` (`KismetMathLibrary.MakeRotator` 0.0 0.0 (.yaw (`self.GetControlRotation`)))) AxisValue))

(event `InputAction|DROP`
  (params (Key :type "Key Structure"))
  (bind _held_item (`self.HELD_ITEM`))
  ;[0.3032 1 0.1758] DROP
  (:`Pressed`
    (if (`self.isHolding`)
      (`|ExecutionSequence`
        (:`then_0`
          (bind (_outhit _returnvalue) (`KismetSystemLibrary.LineTraceSingle` (`self.K2_GetActorLocation`) (- (`self.K2_GetActorLocation`) (0.0 0.0 500.0)) "TraceTypeQuery1"))
          (if _returnvalue
            (`self.K2_DetachFromActor` _held_item "KeepWorld" "KeepWorld" "KeepWorld")
            (`self.K2_SetActorTransform` _held_item (`KismetMathLibrary.MakeTransform` (+ (`.Location` (`GameplayStatics.BreakHitResult` _outhit)) (0.0 0.0 3.0)) (struct :`Roll` -90.0)) false false)
            (set `self.isHolding` false)))))))

(event `InputAxis|LOOK UP/DOWN`
  (params (AxisValue :type "Float (single-precision)"))
  ;[0.1117 1 0.4183] ROTATIONS
  (`self.AddControllerPitchInput` (`KismetMathLibrary.FClamp` AxisValue -5.0 5.0)))

(event `InputAxis|LOOK RIGHT/LEFT`
  (params (AxisValue :type "Float (single-precision)"))
  ;[0.1117 1 0.4183] ROTATIONS
  (`self.AddControllerYawInput` (`KismetMathLibrary.FClamp` AxisValue -5.0 5.0)))

(event `InputAction|CAMERA SWITCH`
  (params (Key :type "Key Structure"))
  (bind _fpscamera (`self.FPSCamera`))
  (bind _tpscamera (`self.TPSCamera`))
  ;[0.1264 0.1388 1] CAMERA SWITCH
  (:`Pressed`
    (`/Engine/EditorBlueprintResources/StandardMacros.FlipFlop`
      (:`A`
        (`ActorComponent.SetActive` _fpscamera true false)
        (`ActorComponent.SetActive` _tpscamera false false)
        (set `self.isFPS` true)
        (set `self.bUseControllerRotationYaw` true))
      (:`B`
        (`ActorComponent.SetActive` _tpscamera true false)
        (`ActorComponent.SetActive` _fpscamera false false)
        (set `self.isFPS` false)
        (set `self.bUseControllerRotationYaw` false)))))

(event `InputAction|JUMP`
  (params (Key :type "Key Structure"))
  ;[0.3121 0.3351 1] SAUT ET S'ACCROUPIR
  (:`Pressed`
    (`self.Jump`)))

(event `InputAction|CROUCH`
  (params (Key :type "Key Structure"))
  ;[0.3121 0.3351 1] SAUT ET S'ACCROUPIR
  (:`Pressed`
    (`self.StartCrouch`))
  (:`Released`
    (`self.StopCrouch`)))

(event `StartCrouch`
  ;[0.2113 0.2598 1] SMOOTH CROUCH
  (set `self.IsCrouched` true)
  (set `CharacterMovementComponent.MaxWalkSpeed` 250.0 (`self.CharacterMovement`)))

(event `StopCrouch`
  ;[0.2113 0.2598 1] SMOOTH CROUCH
  (set `self.IsCrouched` false)
  (set `CharacterMovementComponent.MaxWalkSpeed` 500.0 (`self.CharacterMovement`)))

(fn `decrease life`
  (bind _returnvalue (`KismetMathLibrary.FClamp` (- (`self.Life_Actually`) (`self.Life_decrement`)) 0.0 (`self.Life_base`)))
  (if (not (<= _returnvalue 0.0))
    (set `self.Life_Actually` _returnvalue)))

(fn `Def Base stat Actually`
  (set `self.Life_Actually` (`self.Life_base`)))

(fn `Def init stat perso`
  (set `self.Life_base` 100.0))

(fn `EnterDeathState`
  (bind _returnvalue (`GameplayStatics.GetPlayerController` 0))
  (bind _returnvalue_2 (`|CreateWidget` "/Game/UI/WBP_DeathScreen.WBP_DeathScreen_C" _returnvalue))
  (`UserWidget.AddToViewport` _returnvalue_2 0)
  (`self.DisableInput` self _returnvalue)
  (set `self.isDead` true)
  (`self.EnterRagdollState`)
  (`AIPerceptionStimuliSourceComponent.UnregisterFromSense` (`self.AIPerceptionStimuliSource`) "/Script/AIModule.AISense_Sight")
  (`AIPerceptionStimuliSourceComponent.UnregisterFromPerceptionSystem` (`self.AIPerceptionStimuliSource`)))

(fn `EnterRagdollState`
  (`PrimitiveComponent.SetSimulatePhysics` (`self.Mesh`) true))

(fn `UserConstructionScript`)