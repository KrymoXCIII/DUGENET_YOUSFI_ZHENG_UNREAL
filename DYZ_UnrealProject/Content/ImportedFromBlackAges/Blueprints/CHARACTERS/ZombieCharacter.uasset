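; Zombie enemy character that takes melee hits from DefaultCharacter and can play an attack of its own.
; On actor overlap it checks the player's striking flag and sword hitbox, then subtracts fixed health, playing an impact montage or destroying itself at zero.
; The axe/sword tag sets ActualDamage, but the live path ignores it.
; AttackPlayer plays a montage and uses delays to open and close an IsStriking window.
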(event `self.ReceiveActorBeginOverlap`
  (params (OtherActor :type "Actor Object Reference"))
  (bind _asdefault_character (cast `/Game/Blueprints/CHARACTERS/DefaultCharacter` OtherActor))
  (if (`/Game/Blueprints/CHARACTERS/DefaultCharacter.isStriking` _asdefault_character)
    (if (`PrimitiveComponent.IsOverlappingActor` (`/Game/Blueprints/CHARACTERS/DefaultCharacter.SwordSimulateHitbox` _asdefault_character) self)
      (`|ExecutionSequence`
        (:`then_0`
          (bind _held_item (`/Game/Blueprints/CHARACTERS/DefaultCharacter.HELD_ITEM` _asdefault_character))
          (if (`self.ActorHasTag` _held_item "Axe")
            (set `self.actualDamage` (`self.damageFromAxe`))
            (`KismetSystemLibrary.PrintString` "AXE" true true (struct :`A` 1.0))
            (elif (`self.ActorHasTag` _held_item "Sword")
              (set `self.actualDamage` (`self.damageFromSword`))
              (`KismetSystemLibrary.PrintString` "SWORD" true true (struct :`A` 1.0)))))
        (:`then_1`
          (`/Engine/EditorBlueprintResources/StandardMacros.DoOnce` false :!label _label
            (:`Completed`
              (`GameplayStatics.PlaySound2D` "/Game/EasyBuildingSystem/Audio/Sounds/Interactions/Mining/SFX_Pickaxe_Tool_001.SFX_Pickaxe_Tool_001" 1.0 1.0 0.0 null null)
              (`KismetSystemLibrary.PrintString` "PLAYER ATTACK" true true (struct :`R` 0.006095 :`G` 1.0 :`B` 0.056186 :`A` 1.0))
              (bind _output_get (set `self.ZOMBIEHEALTH` (`KismetMathLibrary.FClamp` (- (`self.ZOMBIEHEALTH`) 20.0) 0.0 100.0)))
              (`KismetSystemLibrary.PrintString` (`KismetStringLibrary.Conv_DoubleToString` _output_get))
              (if (<= (`self.ZOMBIEHEALTH`) 0.0)
                (`KismetSystemLibrary.PrintString` "ZOMBIE IS DEAD")
                (`self.K2_DestroyActor`)
                (else
                  (`self.PlayAnimMontage` "/Game/ANIMS/ZOMBIE/RETARGETED/zombie_impact_Montage.zombie_impact_Montage")
                  (goto _label :!via `Reset`))))))))))

(event `self.ReceiveTick`
  (params (DeltaSeconds :type "Float (single-precision)")))

(event `self.ReceiveBeginPlay`
  (set `self.ZOMBIEHEALTH` 100.0))

(event `Attack Player`
  (`|ExecutionSequence`
    (:`then_0`
      (`|PlayMontage` (`self.Mesh`) "/Game/ANIMS/ZOMBIE/RETARGETED/zombie_attack_MontageATTACK.zombie_attack_MontageATTACK"
        (:`then`
          (cast `/Game/Blueprints/CHARACTERS/DefaultCharacter` (`GameplayStatics.GetPlayerCharacter` 0))
          (`KismetSystemLibrary.Delay` 1.2)
          (set `self.isStriking` false))))
    (:`then_1`
      (`KismetSystemLibrary.Delay` 0.5)
      (set `self.isStriking` true))))

(fn `decrease life`
  (if (<= (`KismetMathLibrary.FClamp` (- 0.0 1.0)) 0.0)
    _))

(fn `Def Base stat Actually`)

(fn `Def init stat perso`)

(fn `EnterDeadState`
  (set `self.isDead` true))

(fn `NewFunction_0`)

(fn `UserConstructionScript`)